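; BP_CardReader is a coloured card reader that unlocks linked doors when a matching key item is held in its scan zone.
; An overlapping actor with the lock tag starts a short timer, which clears the locked state and plays a timeline driving each referenced door's progress.
; End overlap cancels the timer, but checks the tag on the reader itself, not the leaving actor.
; The construction script tints the mesh.
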(event OnComponentBeginOverlap(ScanZone)
  (params (OverlappedComponent :type Primitive%20Component%20Object%20Reference) (OtherActor :type Actor%20Object%20Reference) (OtherComp :type Primitive%20Component%20Object%20Reference) (OtherBodyIndex :type Integer) (bFromSweep :type Boolean) (SweepResult :type Hit%20Result%20Structure%20%28by%20ref%29))
  ;[0.07996 0.1053 0.2865] Begins scanning if the keyitem is in place
  (if (Variables|Default|GetVAR_IsLocked)
    (if (Actor|ActorHasTag OtherActor (Variables|Default|GetVAR_LockTag))
      (bind _returnvalue (Utilities|Time|SetTimerbyEvent (delegate Custom|UnlockDoor) 1.5))
      (Variables|References|SetVAR_TimerReference _returnvalue))))

(event OnComponentEndOverlap(ScanZone)
  (params (OverlappedComponent :type Primitive%20Component%20Object%20Reference) (OtherActor :type Actor%20Object%20Reference) (OtherComp :type Primitive%20Component%20Object%20Reference) (OtherBodyIndex :type Integer))
  ;[0.07996 0.1053 0.2865] Cancels if the key is moved too early
  (if (Actor|ActorHasTag (Variables|Default|GetVAR_LockTag))
    (Utilities|Time|ClearandInvalidateTimerbyHandle (Variables|References|GetVAR_TimerReference))))

(event Custom|UnlockDoor
  ;[0.07996 0.1053 0.2865] Door Unlocking and Opening up
  (Variables|Default|SetVAR_IsLocked false)
  (bind _percentage (Timeline|UnlockTimer Play)
    (:Update
      (for _array_element (Variables|Default|GetVAR_DoorReferences)
        (Class|BPISpinGateSystem|UpdateProgress(Message) _array_element _percentage)))))

(fn ConstructionScript
  (Rendering|Material|SetVectorParameterValueonMaterials (Variables|Default|GetStaticMesh) "Colour" (Math|Conversions|ToVector(LinearColor) (Variables|ScannerSettings|GetVAR_Colour))))