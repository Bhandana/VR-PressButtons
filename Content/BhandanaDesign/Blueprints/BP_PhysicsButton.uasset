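; BP_PhysicsButton is a pressable button that drives the unlock progress of its referenced doors.
; Overlap plays a press timeline that sweeps the button along local Y; completing it plays an unlock timeline feeding progress to each door.
; After release finishes, a non-zero timer schedules relocking by reversing that timeline; a new overlap cancels it.
; The construction script tints the button and derives travel distance from scaled mesh bounds.
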(event OnComponentBeginOverlap(ButtonModel)
  (params (OverlappedComponent :type Primitive%20Component%20Object%20Reference) (OtherActor :type Actor%20Object%20Reference) (OtherComp :type Primitive%20Component%20Object%20Reference) (OtherBodyIndex :type Integer) (bFromSweep :type Boolean) (SweepResult :type Hit%20Result%20Structure%20%28by%20ref%29))
  (CallFunction|ResetTimer)
  (bind (_direction _progress) (Timeline|ButtonProgress Play)
    (:Update
      (Transformation|SetRelativeLocation (Variables|Default|GetButtonModel) (Math|Vector|MakeVector 0.0 (* _progress (Variables|Default|GetVAR_TotalDistance)) 0.0) true false))
    (:Finished
      (if (Utilities|Enum|Equal(Enum) _direction "Forward")
        (CallFunction|UnlockDoor)
        (elif (!= (Variables|Default|GetVAR_Timer) 0.0)
          (CallFunction|BeginCountdown))))))

(event OnComponentEndOverlap(ButtonModel)
  (params (OverlappedComponent :type Primitive%20Component%20Object%20Reference) (OtherActor :type Actor%20Object%20Reference) (OtherComp :type Primitive%20Component%20Object%20Reference) (OtherBodyIndex :type Integer))
  (bind (_direction _progress) (Timeline|ButtonProgress Reverse)
    (:Update
      (Transformation|SetRelativeLocation (Variables|Default|GetButtonModel) (Math|Vector|MakeVector 0.0 (* _progress (Variables|Default|GetVAR_TotalDistance)) 0.0) true false))
    (:Finished
      (if (Utilities|Enum|Equal(Enum) _direction "Forward")
        (CallFunction|UnlockDoor)
        (elif (!= (Variables|Default|GetVAR_Timer) 0.0)
          (CallFunction|BeginCountdown))))))

(event Custom|UnlockDoor
  ;[0.07996 0.1053 0.2865] Door Unlocking and Opening up
  (Variables|Default|SetVAR_IsLocked false)
  (bind _percentage (Timeline|UnlockTimer Play)
    (:Update
      (for _array_element (Variables|Default|GetVAR_DoorReferences)
        (Class|BPISpinGateSystem|UpdateProgress(Message) _array_element _percentage)))))

(event Custom|LockDoor
  ;[0.07996 0.1053 0.2865] Door Unlocking and Opening up
  (Variables|Default|SetVAR_IsLocked true)
  (bind _percentage (Timeline|UnlockTimer Reverse)
    (:Update
      (for _array_element (Variables|Default|GetVAR_DoorReferences)
        (Class|BPISpinGateSystem|UpdateProgress(Message) _array_element _percentage)))))

(event Custom|BeginCountdown
  (bind _returnvalue (Utilities|Time|SetTimerbyEvent (delegate Custom|LockDoor) (Variables|Default|GetVAR_Timer))))

(event Custom|ResetTimer
  (Utilities|Time|ClearandInvalidateTimerbyHandle (stale Custom|BeginCountdown _returnvalue)))

(fn ConstructionScript
  (bind _buttonmodel (Variables|Default|GetButtonModel))
  (bind _max (Components|StaticMesh|GetLocalBounds _buttonmodel))
  (bind _relativescale3d (Variables|/Script/Engine.SceneComponent|GetRelativeScale3D _buttonmodel))
  (bind _returnvalue (* _relativescale3d _max))
  (Rendering|Material|SetVectorParameterValueonMaterials _buttonmodel "Colour" (Math|Conversions|ToVector(LinearColor) (Variables|ScannerSettings|GetVAR_Colour)))
  (Transformation|SetRelativeLocation _buttonmodel (Math|Vector|MakeVector 0.0 (.y _returnvalue) 0.0) false false)
  (Variables|Default|SetVAR_TotalDistance (.y _returnvalue)))